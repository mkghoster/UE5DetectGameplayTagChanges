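; BP_ASCActor is an actor that simulates gameplay tag changes on its Ability System Component, apparently for testing.
; On BeginPlay with authority, a timed Delay sequence applies GE_Tag1, GE_Tag2, then GE_Tag1 again to itself, printing each step.
; It stores the handle of the second GE_Tag1 application and finally removes that effect with all its stacks.
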(event `self.ReceiveBeginPlay`
  (bind _returnvalue (`AbilitySystemBlueprintLibrary.GetAbilitySystemComponent` self))
  (bind _returnvalue_2 (`AbilitySystemBlueprintLibrary.GetAbilitySystemComponent` self))
  (bind _returnvalue_3 (`AbilitySystemBlueprintLibrary.GetAbilitySystemComponent` self))
  (`parent.ReceiveBeginPlay`)
  ;[1 1 1] Simulate gameplay tag changes
  (if (`self.HasAuthority`)
    (`KismetSystemLibrary.Delay` 4.0)
    (`KismetSystemLibrary.PrintString` "Adding Tag1")
    (`AbilitySystemComponent.BP_ApplyGameplayEffectToSelf` _returnvalue_3 "/Game/Blueprints/ASC/GE_Tag1.GE_Tag1_C" 0.0 (`AbilitySystemComponent.MakeEffectContext` _returnvalue_3))
    (`KismetSystemLibrary.Delay` 3.0)
    (`KismetSystemLibrary.PrintString` "Adding Tag2")
    (`AbilitySystemComponent.BP_ApplyGameplayEffectToSelf` _returnvalue "/Game/Blueprints/ASC/GE_Tag2.GE_Tag2_C" 0.0 (`AbilitySystemComponent.MakeEffectContext` _returnvalue))
    (`KismetSystemLibrary.Delay` 3.0)
    (`KismetSystemLibrary.PrintString` "Adding Tag1")
    (bind _returnvalue_4 (`AbilitySystemComponent.BP_ApplyGameplayEffectToSelf` _returnvalue_2 "/Game/Blueprints/ASC/GE_Tag1.GE_Tag1_C" 0.0 (`AbilitySystemComponent.MakeEffectContext` _returnvalue_2)))
    (set `self.Temp` _returnvalue_4)
    (`KismetSystemLibrary.Delay` 3.0)
    (`KismetSystemLibrary.PrintString` "Remove Tag 1")
    (`AbilitySystemComponent.RemoveActiveGameplayEffect` (`AbilitySystemBlueprintLibrary.GetAbilitySystemComponent` self) (`self.Temp`) -1)))

(fn `UserConstructionScript`)