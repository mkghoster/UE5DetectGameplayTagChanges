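; Actor that listens for gameplay tag changes on a target actor's Ability System Component and reports them as debug prints.
; On BeginPlay, only with authority, it starts an async ListenForGameplayTagChange task on TargetActor's ASC, or prints a warning if the target is invalid.
; When a change fires, it prints the tag and its new count, then destroys itself.
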(event `self.ReceiveBeginPlay`
  (`parent.ReceiveBeginPlay`)
  (`/Engine/EditorBlueprintResources/ActorMacros.Switch Has Authority`
    (:`Authority`
      (`/Engine/EditorBlueprintResources/StandardMacros.IsValid` (`self.TargetActor`)
        (:`Is Valid`
          (bind (_tag _newcount) (`AsyncASCGameplayTagChange.ListenForGameplayTagChange` (`AbilitySystemBlueprintLibrary.GetAbilitySystemComponent` (`self.TargetActor`)))
            (:`then`
              (`KismetSystemLibrary.PrintString` "Continue"))
            (:`OnGameplayTagChanged`
              (`KismetSystemLibrary.PrintString` (`KismetStringLibrary.Concat_StrStr` "Gameplay tag changed: " (`BlueprintGameplayTagLibrary.GetDebugStringFromGameplayTag` _tag) ", num: " (`KismetStringLibrary.Conv_IntToString` _newcount)))
              (`self.K2_DestroyActor`))))
        (:`Is Not Valid`
          (`KismetSystemLibrary.PrintString` "Warning: Target ASC Actor is not valid"))))))

(fn `UserConstructionScript`)